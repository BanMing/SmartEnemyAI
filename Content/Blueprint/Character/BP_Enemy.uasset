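; BP_Enemy is an enemy character that plays montages to attack, draw and sheathe a weapon, reporting results through event dispatchers.
; Drawing spawns and attaches a weapon actor at a montage notify, messaging it with the mesh, while sheathing calls destroy on WeaponActor at its notify.
; Montage completion updates the wielding flag and signals weapon readiness; attacks signal their end on completion or interruption.
; Delayed player-chase logic is present but never runs.
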(event `self.ReceiveBeginPlay`
  (set `self.bIsWiedingWeapon` false))

(event `self.BP_OnMoveCompleted`
  (params (MovementResult :type "EPathFollowingResult Enum" :default "Success")))

(event `EnemyInterface.Attack`
  (`|PlayMontage` (`self.Mesh`) (`self.AttackAnim`)
    (:`OnCompleted`
      _)
    (:`OnInterrupted`
      _))
  (`self.OnAttackEnd`))

(event `EnemyInterface.WieldingWeapon`
  (bind _notifyname (`|PlayMontage` (`self.Mesh`) (`self.WieldingWeaponMontage`))
    (:`OnCompleted`
      (set `self.bIsWiedingWeapon` true)
      (`self.OnWeaponReady` true))
    (:`OnNotifyBegin`
      (switch `name` _notifyname
        (:`WieldingWeapon`
          (bind _returnvalue (`|SpawnActorFromClass` (`self.WeaponClass`) (`self.GetTransform`) "Undefined" "MultiplyWithRoot" self null))
          (set `self.WeaponActor` null)
          (`self.K2_AttachToActor` _returnvalue self "None" "KeepRelative" "KeepRelative" "KeepRelative" true)
          (message `WeaponInterface.WieldWeapon` _returnvalue (`self.Mesh`)))))))

(event `EnemyInterface.SheathWeapon`
  (bind _notifyname (`|PlayMontage` (`self.Mesh`) (`self.SheathWeaponMontage`))
    (:`OnCompleted`
      (set `self.bIsWiedingWeapon` false)
      (`self.OnWeaponReady` false))
    (:`OnNotifyBegin`
      (switch `name` _notifyname
        (:`SheathWeapon`
          (`self.K2_DestroyActor` (`self.WeaponActor`)))))))

(fn `IsWiedingWeapon`
  (returns (ReturnValue :type Boolean))
  (return (`self.bIsWiedingWeapon`)))

(fn `UserConstructionScript`)